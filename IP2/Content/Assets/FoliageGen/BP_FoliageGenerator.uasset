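; Foliage scatter actor that, on BeginPlay, places static mesh instances on surfaces within a box sized in the construction script.
; SpawnFoliage gives each key in the Meshes map its own Hierarchical Instanced Static Mesh component, using the value as target count.
; Visibility line traces from GetTraceParams place instances at hits, pitched to follow the surface normal, with attempts capped at twice the target.
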(event `self.ReceiveBeginPlay`
  (`self.SpawnFoliage`))

(fn `SpawnFoliage`
  (locals (SpawnedNumber :type Integer) (Attempts :type Integer))
  (bind (_start _end) (`self.GetTraceParams`))
  (bind _keys (`BlueprintMapLibrary.Map_Keys` (`self.Meshes`)))
  (for _array_element _keys
    (bind (_value _returnvalue) (`BlueprintMapLibrary.Map_Find` (`self.Meshes`) _array_element))
    (if _returnvalue
      (bind _returnvalue_2 (`AddComponent|NODE_AddHierarchicalInstancedStaticMeshComponent-1` :`RelativeTransform` (`self.GetTransform`)))
      (`StaticMeshComponent.SetStaticMesh` _returnvalue_2 _array_element)
      (while (and (< (`local.SpawnedNumber`) _value) (< (`local.Attempts`) (* _value 2)))
        (bind (_outhit _returnvalue_3) (`KismetSystemLibrary.LineTraceSingle` :`Start` _start :`End` _end :`TraceChannel` "TraceTypeQuery1" :`DrawTime` 10.0))
        (`/Engine/EditorBlueprintResources/StandardMacros.IncrementInt` (`local.Attempts`)
          (:`  `
            (if _returnvalue_3
              (bind (_bblockinghit _binitialoverlap _time _distance _location _impactpoint _normal) (`GameplayStatics.BreakHitResult` _outhit))
              (`InstancedStaticMeshComponent.AddInstanceWorldSpace` _returnvalue_2 (`KismetMathLibrary.MakeTransform` _location (`KismetMathLibrary.MakeRotator` (.roll (`KismetMathLibrary.Conv_VectorToRotator` _normal)) (- (.pitch (`KismetMathLibrary.Conv_VectorToRotator` _normal)) 90.0) (.yaw (`KismetMathLibrary.Conv_VectorToRotator` _normal)))))
              (`/Engine/EditorBlueprintResources/StandardMacros.IncrementInt` (`local.SpawnedNumber`))))))
      (set `local.SpawnedNumber` 0)
      (set `local.Attempts` 0)))
  (set `self.RunBuild` false))

(fn `UserConstructionScript`
  (`BoxComponent.SetBoxExtent` (`self.Box`) (`self.BoxExtents`) true))