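; OtterBoat is an actor that moves a boat along the spline of a referenced path actor.
; When active at BeginPlay, it starts the BoatMover timeline from a start offset, with play rate set to the inverse of BoatSpeed, so higher values move it slower.
; Each update maps the timeline alpha to a distance along the spline and applies that point's world location and rotation to the actor.
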(event `self.ReceiveBeginPlay`
  (if (`self.ActiveBoat`)
    (`self.MoveBoat`)))

(event `MoveBoat`
  (bind _returnvalue (`KismetMathLibrary.Lerp` 0.0 (`SplineComponent.GetSplineLength` (`/Game/Blueprints/Path.Spline` (`self.PathRef`))) (`self.Alpha`)))
  (`TimelineComponent.SetPlayRate` (`self.BoatMover`) (/ 1.0 (`self.BoatSpeed`)))
  (`TimelineComponent.SetNewTime` (`self.BoatMover`) (`self.BoatStartOffSet`))
  (bind (_direction _alpha) (`Timeline|BoatMover`)
    (:`Update`
      (set `self.Alpha` _alpha)
      (`self.K2_SetActorLocationAndRotation` (`SplineComponent.GetLocationAtDistanceAlongSpline` (`/Game/Blueprints/Path.Spline` (`self.PathRef`)) _returnvalue "World") (`SplineComponent.GetRotationAtDistanceAlongSpline` (`/Game/Blueprints/Path.Spline` (`self.PathRef`)) _returnvalue "World")))))

(fn `UserConstructionScript`)